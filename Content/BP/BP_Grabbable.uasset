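; Physics object that can be focused and selected, then pushed along a chosen gravity direction.
; Focus toggles the Pick highlight; selection shows the widgets, adds a post-process component, enables physics and allows choosing a direction.
; Once a direction is chosen, Tick clears the effect and widgets, then applies force for Y or Z directions only, holding velocity at the speed limit.
; EDirection2Vector converts all six directions to scaled vectors but is not called here.
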(event `self.ReceiveBeginPlay`
  (`SceneComponent.SetVisibility` (`self.Widget2`) false false)
  (`SceneComponent.SetVisibility` (`self.Widget3`) false false)
  (`SceneComponent.SetVisibility` (`self.Widget`) false false)
  (`SceneComponent.SetVisibility` (`self.Widget1`) false false))

(event `self.ReceiveTick`
  (params (DeltaSeconds :type "Float (single-precision)"))
  (if (`self.HasChooseDirection`)
    (`|ExecutionSequence`
      (:`then_0`
        (`self.Kill PPand Ui`))
      (:`then_1`
        (switch `/Game/BP/E_GravityDirection` (`self.EGravityDirection`)
          (:`NewEnumerator0`
            (if (`self.IsSimulatingGravity`)
              (`self.Add Force` (`self.Dir+Z`))))
          (:`NewEnumerator1`
            (if (`self.IsSimulatingGravity`)
              (`self.Add Force` (`self.Dir-Z`))))
          (:`NewEnumerator4`
            (if (`self.IsSimulatingGravity`)
              (`self.Add Force` (`self.Dir+Y`))))
          (:`NewEnumerator5`
            (if (`self.IsSimulatingGravity`)
              (`self.Add Force` (`self.Dir-Y`)))))))))

(event `CE_Focus`
  (`SceneComponent.SetVisibility` (`self.Pick`) true false)
  (set `self.CanSelete` true))

(event `CE_UnFocus`
  (`SceneComponent.SetVisibility` (`self.Pick`) false false)
  (set `self.CanSelete` false))

(event `CE_Seleted`
  (`SceneComponent.SetVisibility` (`self.Widget`) true false)
  (`SceneComponent.SetVisibility` (`self.Widget1`) true false)
  (`SceneComponent.SetVisibility` (`self.Widget2`) true false)
  (`SceneComponent.SetVisibility` (`self.Pick`) true false)
  (`SceneComponent.SetVisibility` (`self.Widget3`) true false)
  (bind _returnvalue (`AddComponent|NODE_AddPostProcessComponent-0`))
  (set `self.CanChooseDirection` true)
  (set `self.PP` _returnvalue)
  (`PrimitiveComponent.SetSimulatePhysics` (`self.Normal`) true))

(event `CE_UnSeleted`
  (`SceneComponent.SetVisibility` (`self.Widget`) false false)
  (`SceneComponent.SetVisibility` (`self.Widget1`) false false)
  (`SceneComponent.SetVisibility` (`self.Widget2`) false false)
  (`SceneComponent.SetVisibility` (`self.Pick`) false false)
  (`SceneComponent.SetVisibility` (`self.Widget3`) false false))

(fn `Add Force`
  (params (Direction :type "Vector Structure"))
  (bind _returnvalue (`PrimitiveComponent.GetPhysicsLinearVelocity` (`self.Normal`) "None"))
  (if (>= (`KismetMathLibrary.VSize` _returnvalue) (`self.MaxSpeedLimit`))
    (`PrimitiveComponent.SetPhysicsLinearVelocity` (`self.Normal`) _returnvalue false "None") ; 超速了就设置速度不变
    (else
      (`PrimitiveComponent.AddForce` (`self.Normal`) (* Direction (`self.ForceStrength`)) "None" false) ; 没超速就继续加速
    )))

(fn `EDirection2Vector`
  (params (`Gravity Direction` :type "/Game/BP/E_GravityDirection Enum" :default "NewEnumerator0"))
  (returns (GravityDirection :type "Vector Structure"))
  (switch `/Game/BP/E_GravityDirection` `Gravity Direction`
    (:`NewEnumerator0`
      (return (* (`self.GravityStrength`) (`KismetMathLibrary.MakeVector` 0.0 0.0 1.0))))
    (:`NewEnumerator1`
      (return (* (`self.GravityStrength`) (`KismetMathLibrary.MakeVector` 0.0 0.0 -1.0))))
    (:`NewEnumerator2`
      (return (* (`self.GravityStrength`) (`KismetMathLibrary.MakeVector` 1.0))))
    (:`NewEnumerator3`
      (return (* (`self.GravityStrength`) (`KismetMathLibrary.MakeVector` -1.0))))
    (:`NewEnumerator4`
      (return (* (`self.GravityStrength`) (`KismetMathLibrary.MakeVector` 0.0 1.0))))
    (:`NewEnumerator5`
      (return (* (`self.GravityStrength`) (`KismetMathLibrary.MakeVector` 0.0 -1.0))))))

(fn `Kill PPand Ui`
  (bind _pp (`self.PP`))
  (`|ExecutionSequence`
    (:`then_0`
      (`/Engine/EditorBlueprintResources/StandardMacros.IsValid` _pp
        (:`Is Valid`
          (`ActorComponent.K2_DestroyComponent` _pp))))
    (:`then_1`
      (`SceneComponent.SetVisibility` (`self.Widget1`) false false)
      (`SceneComponent.SetVisibility` (`self.Widget2`) false false)
      (`SceneComponent.SetVisibility` (`self.Widget3`) false false)
      (`SceneComponent.SetVisibility` (`self.Widget`) false false))))

(fn `UserConstructionScript`)